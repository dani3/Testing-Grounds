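; AI behavior tree task that selects the next patrol waypoint for a ThirdPersonCharacter.
; It reads the character's patrol points and writes the one at blackboard Index to Waypoint.
; It then stores (Index % count) + 1 back, which cycles 1 to count rather than zero-based, so it reaches an out-of-range index.
; The task always finishes successfully once executed.
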(event `self.ReceiveExecuteAI`
  (params (OwnerController :type "AIController Object Reference") (ControlledPawn :type "Pawn Object Reference"))
  (`self.Get Patrol Points` ControlledPawn)
  (bind _index (`self.Select Next Waypoint`))
  (`self.Cycle Index` _index)
  (`self.FinishExecute` true))

(fn `Cycle Index`
  (params (Index :type Integer))
  (`BTFunctionLibrary.SetBlackboardValueAsInt` (`self.Index`) (+ (mod Index (`KismetArrayLibrary.Array_Length` (`self.Patrol Points`))) 1)))

(fn `Get Patrol Points`
  (params (Pawn :type "Object Object Reference"))
  (bind _asthird_person_character (cast `/Game/ThirdPersonCPP/Blueprints/ThirdPersonCharacter` Pawn))
  (set `self.Patrol Points` (`/Game/ThirdPersonCPP/Blueprints/ThirdPersonCharacter.Patrol Point` _asthird_person_character)))

(fn `Select Next Waypoint`
  (returns (Index :type Integer))
  (bind _returnvalue (`BTFunctionLibrary.GetBlackboardValueAsInt` (`self.Index`)))
  (`BTFunctionLibrary.SetBlackboardValueAsObject` (`self.Waypoint`) (`|GetArrayItem` (`self.Patrol Points`) _returnvalue))
  (return _returnvalue))